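; BP_AOE_Blast_Base is a base Blueprint for blast-type area-of-effect actors, adding a visual effect and self-cleanup to an inherited Trigger event.
; Trigger runs the parent logic, then spawns the BlastEffect particle system attached to the root component.
; The actor destroys itself when that particle system finishes, or after a short delay if no valid effect is set.
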(event Custom|SystemFinished
  (params (PSystem :type Particle%20System%20Component%20Object%20Reference))
  (Actor|DestroyActor))

(event Custom|SpawnBlastEffect
  (bind _blast_effect (Variables|Default|GetBlast%20Effect)
    (:then
      (bind _returnvalue (Effects|SpawnEmitterAttached _blast_effect (Variables|Default|GetDefaultSceneRoot) "None"))
      (EventDispatchers|BindEventtoOnSystemFinished _returnvalue (delegate Custom|SystemFinished)))
    (:else
      (Utilities|FlowControl|Delay 1.0)
      (Actor|DestroyActor))))

(event EventBeginPlay
  (|CallParentFunction) ; This node is disabled and will not be called.\nDrag off pins to build functionality.
)

(event Collision|EventActorBeginOverlap
  (params (OtherActor :type Actor%20Object%20Reference)))

(event EventTick
  (params (DeltaSeconds :type Float%20%28single-precision%29)))

(event EventTrigger
  (|CallParentFunction)
  (CallFunction|SpawnBlastEffect))

(fn ConstructionScript
  (|CallParentFunction))