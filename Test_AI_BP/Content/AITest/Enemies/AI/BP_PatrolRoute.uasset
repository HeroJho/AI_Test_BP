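; BP_PatrolRoute is a patrol path for enemy AI, defined by the points of a PatrolRoute spline.
; It tracks a current point index and exposes that point's world position through a getter.
; IncrementPatrolRoute steps the index by a direction value that flips at the first and last points, so the route is traversed back and forth rather than looped.
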(event Custom|IncrementPatrolRoute
  (bind _output_get (Variables|Default|SetPartrolIndex (+ (Variables|Default|GetPartrolIndex) (Variables|Default|GetDirection))))
  (if (== _output_get (- (Spline|GetNumberOfSplinePoints (Variables|Default|GetPatrolRoute)) 1))
    (Variables|Default|SetDirection -1)
    (elif (== (Variables|Default|GetPartrolIndex) 0)
      (Variables|Default|SetDirection 1))))

(fn ConstructionScript)

(fn GetSplinePointasWorldPosition
  (return (Spline|GetLocationatSplinePoint (Variables|Default|GetPatrolRoute) (Variables|Default|GetPartrolIndex) "World")))