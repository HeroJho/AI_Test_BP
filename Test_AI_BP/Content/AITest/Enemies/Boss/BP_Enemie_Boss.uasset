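; Boss enemy character, a child of a base enemy Blueprint, that fights with a sword and has a large health pool set on construction.
; It spawns the sword on BeginPlay, attaches it to its hand socket, and fires equip or unequip notifications one tick after each weapon change.
; AttackCombo1 passes montage and damage info to the attacks component for a melee strike.
; SetMovementSpeed maps movement states to walk speeds.
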(event Custom|AttackCombo1
  (params (AttackTarget :type Actor%20Object%20Reference))
  (Default|PrimaryMeleeAttack (Variables|Default|GetBPC_Attacks) (Utilities|Struct|MakeS_AttackInfo AttackTarget "/Game/AITest/Animations/Melee/AM_Attack.AM_Attack" (Utilities|Struct|MakeS_DamageInfo 1e+01 "NewEnumerator1" "NewEnumerator1" false true true)) 4e+01 2.5e+02))

(event EventBeginPlay
  (|CallParentFunction)
  (CallFunction|EquipWeapon))

(event Collision|EventActorBeginOverlap
  (params (OtherActor :type Actor%20Object%20Reference)))

(event EventTick
  (params (DeltaSeconds :type Float%20%28single-precision%29)))

(event EventEquipWeapon
  ;[1 1 1] Weapon
  (bind _returnvalue (Game|SpawnActorfromClass "/Game/AITest/Weapons/BP_Weapon_Sword.BP_Weapon_Sword_C" (Math|Transform|MakeTransform "0, 0, 0" "0, 0, 0" "1.000000,1.000000,1.000000") "Undefined" "MultiplyWithRoot" 0 0))
  (bind _output_get (Variables|Default|SetWeaponActor _returnvalue))
  (Transformation|AttachComponentToComponent _output_get (Variables|Character|GetMesh) "hand_rSocket" "SnapToTarget" "SnapToTarget" "SnapToTarget" true)
  (Variables|Default|SetIsWieldingWeapon true)
  (Utilities|FlowControl|DelayUntilNextTick)
  (Default|CallOnWeaponEquipped))

(event EventUnequipWeapon
  ;[1 1 1] Weapon
  (Actor|DestroyActor (Variables|Default|GetWeaponActor))
  (Variables|Default|SetIsWieldingWeapon false)
  (Utilities|FlowControl|DelayUntilNextTick)
  (Default|CallOnWeaponUnquipped))

(fn ConstructionScript
  (bind _bpc_damagesystem (Variables|Default|GetBPC_DamageSystem))
  (|CallParentFunction)
  (bind _output_get (Variables|/Game/AITest/Components/DamageSystem/BPC_DamageSystem.BPC_DamageSystem_C|SetMaxHealth _bpc_damagesystem 1e+03))
  (Variables|/Game/AITest/Components/DamageSystem/BPC_DamageSystem.BPC_DamageSystem_C|SetHealth _bpc_damagesystem _output_get))

(fn SetMovementSpeed
  (params (Speed :type E_MovementSpeed%20Enum :default "NewEnumerator0"))
  (bind _output_get (Variables|/Script/Engine.CharacterMovementComponent|SetMaxWalkSpeed (Variables|Character|GetCharacterMovement) (Utilities|Select :Index Speed :NewEnumerator0 0.0 :NewEnumerator1 1e+02 :NewEnumerator2 2e+02 :NewEnumerator3 3.5e+02)))
  (return _output_get))