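; Ranged enemy character that wields a rifle and shoots at the attack target held by its AI controller.
; On BeginPlay it spawns the rifle and attaches it to the hand socket.
; Attack plays a firing montage whose notify has the attacks component fire a bullet from the weapon toward the target, signaling attack end on completion or interruption.
; It also maps movement states to walk speeds and supplies ideal attack and defend ranges.
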(event EventBeginPlay
  (|CallParentFunction)
  (CallFunction|EquipWeapon))

(event EventEquipWeapon
  (bind _returnvalue (Game|SpawnActorfromClass "/Game/AITest/Weapons/BP_Weapon_Rifle.BP_Weapon_Rifle_C" (Math|Transform|MakeTransform "0, 0, 0") "Undefined" "MultiplyWithRoot" 0 0))
  (bind _output_get (Variables|Default|SetWeaponActor _returnvalue))
  (Transformation|AttachComponentToComponent _output_get (Variables|Character|GetMesh) "hand_rSocket_rifle" "SnapToTarget" "SnapToTarget" "SnapToTarget" true)
  (Variables|Default|SetIsWieldingWeapon true)
  (Default|CallOnWeaponEquipped))

(event EventAttack
  (Variables|Default|SetAttacking true)
  (bind _notifyname (Animation|Montage|PlayMontage (Variables|Character|GetMesh) "/Game/AITest/Animations/Rifle/AM_FiringRifle.AM_FiringRifle")
    (:OnCompleted
      (Default|CallOnAttackEnd :!label _label)
      (Variables|Default|SetAttacking false))
    (:OnInterrupted
      (goto _label))
    (:OnNotifyBegin
      (switch name _notifyname
        (:Fire
          (bind _asaic_enemy_base (Utilities|Casting|CastToAIC_Enemy_Base (AI|GetAIController self)))
          (bind _attacktarget (Variables|/Game/AITest/Enemies/AI/AIC_Enemy_Base.AIC_Enemy_Base_C|GetAttackTarget _asaic_enemy_base)
            (:then
              (Default|FireBullet (Variables|Default|GetBPC_Attacks) (Transformation|GetActorLocation (Variables|Default|GetWeaponActor)) (Transformation|GetActorLocation _attacktarget) (Utilities|Struct|MakeS_DamageInfo 15.0 "NewEnumerator2" "NewEnumerator0" false true)))
            (:else)))))))

(fn ConstructionScript
  (|CallParentFunction))

(fn SetMovementSpeed
  (params (Speed :type E_MovementSpeed%20Enum :default "NewEnumerator0"))
  (Variables|/Script/Engine.CharacterMovementComponent|SetMaxWalkSpeed (Variables|Character|GetCharacterMovement) (Utilities|Select :Index Speed :NewEnumerator0 0.0 :NewEnumerator1 2e+02 :NewEnumerator2 3e+02 :NewEnumerator3 5e+02))
  (return 0.0))

(fn GetIdealRange
  (return 6e+02 6e+02))