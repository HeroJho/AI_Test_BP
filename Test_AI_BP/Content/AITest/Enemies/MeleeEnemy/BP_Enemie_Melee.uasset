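; Sword-wielding melee enemy character with short-range, jump and spinning attacks, weapon equip/unequip and chance-based blocking.
; Attack montage notifies drive forward sphere-trace damage, predictive arced leaps at the target, and a timeline mesh spin that chases the target before an AOE slash.
; BPC_DamageSystem handles damage and blocks, with interruption disabled during attacks.
; Events report attack, equip and block completion, and GetIdealRange supplies attack and defend radii.
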(event OnBlock(BPC_DamageSystem)
  (params (CanBeParried :type Boolean))
  ;[1 1 1] Blocking
  (Variables|Default|SetBlockingState "NewEnumerator2")
  (Utilities|Time|ClearandInvalidateTimerbyHandle (Variables|Default|GetHoldBlockTimer))
  (Animation|Montage|PlayMontage (Variables|Character|GetMesh) "/Game/AITest/Animations/Melee/AM_BlockReact.AM_BlockReact"
    (:OnCompleted
      _)
    (:OnInterrupted
      _))
  (CallFunction|EndBlock))

(event Custom|EndBlock
  ;[1 1 1] Blocking
  (Variables|Default|SetBlockingState "NewEnumerator0")
  (Variables|/Game/AITest/Components/DamageSystem/BPC_DamageSystem.BPC_DamageSystem_C|SetIsBlocking (Variables|Default|GetBPC_DamageSystem) false)
  (Default|CallOnBlockEnded))

(event Custom|Start%20Block
  ;[1 1 1] Blocking
  (Components|Movement|StopMovementImmediately (Variables|Character|GetCharacterMovement))
  (Variables|Default|SetBlockingState "NewEnumerator1")
  (Variables|/Game/AITest/Components/DamageSystem/BPC_DamageSystem.BPC_DamageSystem_C|SetIsBlocking (Variables|Default|GetBPC_DamageSystem) true)
  (Utilities|Time|ClearandInvalidateTimerbyHandle (Variables|Default|GetHoldBlockTimer))
  (bind _returnvalue (Utilities|Time|SetTimerbyEvent (EventDispatchers|CreateEvent :!event Custom|EndBlock) 2.0))
  (Variables|Default|SetHoldBlockTimer _returnvalue))

(event Custom|StopSpinning
  ;[1 1 1] Attack Helpers
  (Audio|Components|Audio|Stop (Variables|Default|GetSpinMeshTimeline))
  (Transformation|SetRelativeRotation (Variables|Character|GetMesh) (Variables|Default|GetMeshRotationBeforeSpin) false false))

(event Custom|ChaseAttackTarget
  (params (AttackTarget :type Actor%20Object%20Reference))
  ;[1 1 1] Attack Helpers
  (AI|AIMoveTo self "0, 0, 0" AttackTarget 5e+01 false
    (:OnSuccess
      (Utilities|FlowControl|Delay 0.1)
      (if (Variables|Default|GetAttacking)
        (CallFunction|ChaseAttackTarget AttackTarget)))))

(event Custom|AOEDamageActor
  (params (Actor :type Actor%20Object%20Reference))
  ;[1 1 1] Attack Helpers
  (if (== Actor (stale Custom|AOESlash AttackTarget))
    (Class|BPIDamagable|TakeDamage(Message) Actor (Utilities|Struct|MakeS_DamageInfo 1e+02 "NewEnumerator1") self)))

(event Custom|SphereTraceDamage
  (bind _returnvalue (Transformation|GetActorLocation))
  ;[1 1 1] Attack Helpers
  (bind (_outhits _returnvalue_2) (Collision|MultiSphereTraceForObjects _returnvalue (+ _returnvalue (* (Transformation|GetActorForwardVector) 2e+02)) 0.0 (Utilities|Array|MakeArray "ObjectTypeQuery3") false 0 "None"))
  (if _returnvalue_2
    (Default|DamageAllNonTeamMebers (Variables|Default|GetBPC_Attacks) _outhits (Utilities|Struct|MakeS_DamageInfo 3e+01 "NewEnumerator1"))))

(event Custom|ShortRangeAttack
  (params (AttackTarget :type Actor%20Object%20Reference))
  ;[1 1 1] Sword Slash
  (|CallParentFunction AttackTarget)
  (bind _notifyname (Animation|Montage|PlayMontage (Variables|Character|GetMesh) "/Game/AITest/Animations/Melee/AM_Attack.AM_Attack")
    (:then
      (Variables|/Game/AITest/Components/DamageSystem/BPC_DamageSystem.BPC_DamageSystem_C|SetIsInterruptible (Variables|Default|GetBPC_DamageSystem) false))
    (:OnCompleted
      (Variables|/Game/AITest/Components/DamageSystem/BPC_DamageSystem.BPC_DamageSystem_C|SetIsInterruptible (Variables|Default|GetBPC_DamageSystem) true :!label _label)
      (CallFunction|AttackEnd AttackTarget))
    (:OnInterrupted
      (goto _label))
    (:OnNotifyBegin
      (switch name _notifyname
        (:Attack
          (CallFunction|SphereTraceDamage))))))

(event Custom|LongRangeAttack
  (params (AttackTarget :type Actor%20Object%20Reference))
  ;[1 1 1] Sword Slash
  (|CallParentFunction AttackTarget)
  (bind _notifyname (Animation|Montage|PlayMontage (Variables|Character|GetMesh) "/Game/AITest/Animations/Melee/AM_SwordJumpAttack.AM_SwordJumpAttack")
    (:then
      (Variables|/Game/AITest/Components/DamageSystem/BPC_DamageSystem.BPC_DamageSystem_C|SetIsInterruptible (Variables|Default|GetBPC_DamageSystem) false))
    (:OnCompleted
      (Variables|/Game/AITest/Components/DamageSystem/BPC_DamageSystem.BPC_DamageSystem_C|SetIsInterruptible (Variables|Default|GetBPC_DamageSystem) true :!label _label)
      (CallFunction|AttackEnd AttackTarget))
    (:OnInterrupted
      (goto _label))
    (:OnNotifyBegin
      (switch name _notifyname
        (:Slash
          (CallFunction|SphereTraceDamage))
        (:Jump
          (CallFunction|JumptoAttackTarget AttackTarget))))))

(event Custom|JumpToAttackTarget
  (params (Attack%20Target :type Actor%20Object%20Reference))
  ;[1 1 1] Attack Helpers
  (bind _location (CallFunction|CalculateFutureActorLocation Attack%20Target 1.0))
  (bind _outlaunchvelocity (Game|SuggestProjectileVelocityCustomArc (Transformation|GetActorLocation) (Math|Vector|MakeVector (.x _location) (.y _location) (+ (.z _location) 1e+02)) 0.0 0.5))
  (Character|LaunchCharacter _outlaunchvelocity true true)
  (EventDispatchers|BindEventtoLandedDelegate (delegate Custom|OnLand)))

(event Custom|OnLand
  (params (Hit :type Hit%20Result%20Structure%20%28by%20ref%29))
  ;[1 1 1] Attack Helpers
  (EventDispatchers|UnbindEventfromLandedDelegate (delegate Custom|OnLand))
  (Components|Movement|StopMovementImmediately (Variables|Character|GetCharacterMovement)))

(event Custom|SpinningAttack
  (params (AttackTarget :type Actor%20Object%20Reference))
  ;[1 1 1] Sword Slash
  (|CallParentFunction AttackTarget)
  (bind _notifyname (Animation|Montage|PlayMontage (Variables|Character|GetMesh) "/Game/AITest/Animations/Melee/AM_SpinAttack.AM_SpinAttack")
    (:then
      (Variables|/Game/AITest/Components/DamageSystem/BPC_DamageSystem.BPC_DamageSystem_C|SetIsInterruptible (Variables|Default|GetBPC_DamageSystem) false))
    (:OnCompleted
      (Variables|/Game/AITest/Components/DamageSystem/BPC_DamageSystem.BPC_DamageSystem_C|SetIsInterruptible (Variables|Default|GetBPC_DamageSystem) true :!label _label)
      (CallFunction|AttackEnd AttackTarget)
      (CallFunction|StopSpinning))
    (:OnInterrupted
      (goto _label))
    (:OnNotifyBegin
      (switch name _notifyname
        (:Slash
          (CallFunction|SphereTraceDamage))
        (:Spin
          (CallFunction|SpinMesh)
          (CallFunction|ChaseAttackTarget AttackTarget))
        (:AOESlash
          (CallFunction|AOESlash AttackTarget))))))

(event Custom|AOESlash
  (params (AttackTarget :type Actor%20Object%20Reference))
  ;[1 1 1] Attack Helpers
  (bind _returnvalue (Game|SpawnActorfromClass "/Game/AITest/AOE/BP_AOE_Base.BP_AOE_Base_C" (Math|Transform|MakeTransform (Transformation|GetActorLocation) "0, 0, 0" "1.000000,1.000000,1.000000") "Undefined" "MultiplyWithRoot" 0 true false false self))
  (Variables|/Game/AITest/AOE/BP_AOE_Base.BP_AOE_Base_C|SetRadius _returnvalue 3e+02)
  (EventDispatchers|BindEventtoOnAOEOverlapActor _returnvalue (delegate Custom|AOEDamageActor))
  (Default|Trigger _returnvalue))

(event Custom|SpinMesh
  ;[1 1 1] Attack Helpers
  (Variables|Default|SetMeshRotationBeforeSpin (Variables|/Script/Engine.SceneComponent|GetRelativeRotation (Variables|Character|GetMesh)))
  (bind _zrotationalpha (Timeline|SpinMeshTimeline PlayFromStart)
    (:Update
      (Transformation|SetRelativeRotation (Variables|Character|GetMesh) (Math|Rotator|MakeRotator (.roll (Variables|Default|GetMeshRotationBeforeSpin)) (.pitch (Variables|Default|GetMeshRotationBeforeSpin)) (Math|Float|Lerp (.yaw (Variables|Default|GetMeshRotationBeforeSpin)) (+ (.yaw (Variables|Default|GetMeshRotationBeforeSpin)) (|(360*12))) _zrotationalpha)) false false))))

(event EventBeginPlay
  (|CallParentFunction) ; This node is disabled and will not be called.\nDrag off pins to build functionality.
)

(event EventEquipWeapon
  ;[1 1 1] Equip Or Unequip Weapon
  (bind _notifyname (Animation|Montage|PlayMontage (Variables|Character|GetMesh) "/Game/AITest/Animations/Melee/AM_WieldSworld.AM_WieldSworld")
    (:OnCompleted
      (Default|CallOnWeaponEquipped))
    (:OnNotifyBegin
      (switch name _notifyname
        (:WieldTiming
          (bind _returnvalue (Game|SpawnActorfromClass "/Game/AITest/Weapons/BP_Weapon_Sword.BP_Weapon_Sword_C" (Transformation|GetActorTransform) "Undefined" "MultiplyWithRoot" 0 0))
          (bind _output_get (Variables|Default|SetWeaponActor _returnvalue))
          (Transformation|AttachComponentToComponent _output_get (Variables|Character|GetMesh) "hand_rSocket" "SnapToTarget" "SnapToTarget" "SnapToTarget" true)
          (Variables|Default|SetIsWieldingWeapon true))))))

(event EventUnequipWeapon
  ;[1 1 1] Equip Or Unequip Weapon
  (bind _notifyname (Animation|Montage|PlayMontage (Variables|Character|GetMesh) "/Game/AITest/Animations/Melee/AM_Sheath_Sword.AM_Sheath_Sword")
    (:OnCompleted
      (Default|CallOnWeaponUnquipped))
    (:OnNotifyBegin
      (switch name _notifyname
        (:DropSword
          (Actor|DestroyActor (Variables|Default|GetWeaponActor))
          (Variables|Default|SetIsWieldingWeapon false))))))

(event EventAttack
  (params (AttackTarget :type Actor%20Object%20Reference))
  ;[1 1 1] Sword Slash
)

(fn ConstructionScript
  (|CallParentFunction)
  (Variables|Default|SetMeshRotationBeforeSpin (Variables|/Script/Engine.SceneComponent|GetRelativeRotation (Variables|Character|GetMesh))))

(fn TakeDamage
  (params (DamageInfo :type S%20Damage%20Info%20Structure) (Causer :type Actor%20Object%20Reference))
  (if (Utilities|Struct|BreakS_DamageInfo DamageInfo)
    (CallFunction|TrytoBlock))
  (bind _wasdamaged (Default|TakeDamage (Variables|Default|GetBPC_DamageSystem) DamageInfo Causer))
  (return _wasdamaged))

(fn TrytoBlock
  (if (<= (Math|Random|RandomFloat) (Variables|Default|GetBlockChance))
    (CallFunction|StartBlock)))

(fn GetIdealRange
  (return 2e+02 4e+02))

(fn CalculateFutureActorLocation
  (params (Actor :type Actor%20Object%20Reference) (Time :type Float%20%28double-precision%29))
  (return (+ (Transformation|GetActorLocation Actor) (* (* (Transformation|GetVelocity Actor) "1.000000,1.000000,0.000000") Time))))