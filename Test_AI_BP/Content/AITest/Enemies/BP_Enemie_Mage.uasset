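; Mage enemy character with a ranged spell attack, a teleport and a self-heal, plus its own attack and defend ranges.
; The attack montage's notify fires a spell from the left hand through BPCAttacks.
; Teleport is faked with invisible high-speed AIMoveTo flight that ignores pawns and trails a particle effect.
; Healing spawns a ground-traced AOE actor that heals only the mage, and dispatchers signal when teleport and heal end.
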(event Custom|Teleport
  (params (Location :type Vector))
  (bind _charactermovement (Variables|Character|GetCharacterMovement))
  ;[1 1 1] Teleport
  (if (Variables|Default|GetIsTeleporting)
    (Utilities|FlowControl|DelayUntilNextTick)
    (Default|CallOnTeleportEnd)
    (else
      (Variables|Default|SetIsTeleporting true)
      (Pawn|Components|CharacterMovement|SetMovementMode _charactermovement "MOVE_Flying" 0)
      (Variables|/Script/Engine.CharacterMovementComponent|SetMaxFlySpeed _charactermovement 5e+03)
      (Variables|/Script/Engine.CharacterMovementComponent|SetMaxAcceleration _charactermovement 99999.0)
      (Rendering|SetVisibility (Variables|Character|GetMesh) false true)
      (Collision|SetCollisionResponsetoChannel (Variables|Default|GetCapsuleComponent) "ECC_Pawn" "ECR_Ignore")
      (bind _returnvalue (Effects|SpawnEmitterAttached "/Game/Resources/InfinityBladeEffects/Effects/FX_Monsters/FX_Monster_FrostGiant/ICE/P_TraceMagic_Trail_Ice.P_TraceMagic_Trail_Ice" (Variables|Character|GetMesh) "spine_01"))
      (Variables|Default|SetTeleportTrailEffect _returnvalue)
      (Animation|StopAnimMontage 0)
      (AI|AIMoveTo self Location 0 5.0 false
        (:OnSuccess
          _)
        (:OnFail
          _))
      (CallFunction|TeleportEnd))))

(event Custom|TeleportEnd
  (bind _charactermovement (Variables|Character|GetCharacterMovement))
  ;[1 1 1] Teleport
  (Components|Movement|StopMovementImmediately _charactermovement)
  (Pawn|Components|CharacterMovement|SetMovementMode _charactermovement "MOVE_Walking" 0)
  (Variables|/Script/Engine.CharacterMovementComponent|SetMaxAcceleration _charactermovement 1.5e+03)
  (Rendering|SetVisibility (Variables|Character|GetMesh) true true)
  (Collision|SetCollisionResponsetoChannel (Variables|Default|GetCapsuleComponent) "ECC_Pawn" "ECR_Block")
  (Default|CallOnTeleportEnd)
  (Utilities|FlowControl|Delay 0.5)
  (Variables|Default|SetIsTeleporting false)
  (bind _teleporttraileffect (Variables|Default|GetTeleportTrailEffect)
    (:then
      (Components|DestroyComponent _teleporttraileffect))
    (:else)))

(event Custom|HealOverTimeEnded
  (Default|CallOnHealoverTimeEnd)
  (bind _aoehealactor (Variables|Default|GetAOEHealActor)
    (:then
      (Actor|DestroyActor _aoehealactor))
    (:else)))

(event Custom|HealOverTime
  (bind _returnvalue (Transformation|GetActorLocation))
  (Animation|Montage|PlayMontage (Variables|Character|GetMesh) "/Game/AITest/Animations/Mage/AM_Heal.AM_Heal"
    (:then
      (bind (_outhit _returnvalue_2) (Collision|LineTraceByChannel _returnvalue (* _returnvalue "1.000000,1.000000,-1000.000000") "TraceTypeQuery1" false (Utilities|Array|MakeArray self) "None"))
      (if _returnvalue_2
        (bind _returnvalue_3 (Game|SpawnActorfromClass "/Game/AITest/AOE/OverTime/BP_AOE_Heal.BP_AOE_Heal_C" (Math|Transform|MakeTransform (.Location (Collision|BreakHitResult _outhit)) "0, 0, 0" "1.000000,1.000000,1.000000") "Undefined" "MultiplyWithRoot" 0 0.5 1e+01 false true true 0))
        (bind _output_get (Variables|Default|SetAOEHealActor _returnvalue_3))
        (EventDispatchers|BindEventtoOnAOEOverlapActor _output_get (delegate Custom|OnHealTarget))
        (else
          (Animation|StopAnimMontage 0))))
    (:OnCompleted
      (CallFunction|HealOverTimeEnded :!label _label))
    (:OnInterrupted
      (goto _label))))

(event Custom|OnHealTarget
  (params (Actor :type Actor%20Object%20Reference))
  (if (== Actor self)
    (Class|BPIDamagable|Heal(Message) Actor 1e+01)))

(event EventBeginPlay
  (|CallParentFunction) ; This node is disabled and will not be called.\nDrag off pins to build functionality.
)

(event Collision|EventActorBeginOverlap
  (params (OtherActor :type Actor%20Object%20Reference)))

(event EventTick
  (params (DeltaSeconds :type Float%20%28single-precision%29)))

(event EventAttack
  (params (AttackTarget :type Actor%20Object%20Reference))
  (|CallParentFunction AttackTarget)
  (bind _notifyname (Animation|Montage|PlayMontage (Variables|Character|GetMesh) "/Game/AITest/Animations/Mage/AM_MagicAttack.AM_MagicAttack")
    (:OnCompleted
      (CallFunction|AttackEnd AttackTarget :!label _label))
    (:OnInterrupted
      (goto _label))
    (:OnNotifyBegin
      (switch name _notifyname
        (:Fire
          (Default|MagicSpell (Variables|Default|GetBPC_Attacks) (Math|Transform|MakeTransform (Transformation|GetSocketLocation (Variables|Character|GetMesh) "hand_l") "0, 0, 0" "1.000000,1.000000,1.000000") AttackTarget (Utilities|Struct|MakeS_DamageInfo 2e+01 "NewEnumerator2")))))))

(fn ConstructionScript
  (|CallParentFunction))

(fn GetIdealRange
  (return 5e+02 7e+02))