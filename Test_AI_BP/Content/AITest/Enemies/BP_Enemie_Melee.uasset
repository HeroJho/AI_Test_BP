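; BP_Enemie_Melee is a sword-wielding melee enemy that implements attack, equip and unequip events.
; Montage notifies time the gameplay: a forward sphere trace that damages pawns, spawning the sword onto the hand socket, and destroying it on sheathe.
; The damage system is set non-interruptible during attacks and restored when the montage completes or is interrupted.
; Dispatchers announce when attacks end and weapon changes complete.
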(event EventBeginPlay
  (|CallParentFunction) ; This node is disabled and will not be called.\nDrag off pins to build functionality.
)

(event EventEquipWeapon
  (bind _notifyname (Animation|Montage|PlayMontage (Variables|Character|GetMesh) "/Game/AITest/Enemies/AI/Animations/Melee/AM_WieldSworld.AM_WieldSworld")
    (:OnCompleted
      (Default|CallOnWeaponEquipped))
    (:OnNotifyBegin
      (switch name _notifyname
        (:WieldTiming
          (bind _returnvalue (Game|SpawnActorfromClass "/Game/AITest/Weapons/BP_Weapon_Sword.BP_Weapon_Sword_C" (Transformation|GetActorTransform) "Undefined" "MultiplyWithRoot" 0 0))
          (bind _output_get (Variables|Default|SetWeaponActor _returnvalue))
          (Transformation|AttachComponentToComponent _output_get (Variables|Character|GetMesh) "hand_rSocket" "SnapToTarget" "SnapToTarget" "SnapToTarget" true)
          (Variables|Default|SetIsWieldingWeapon true))))))

(event EventUnequipWeapon
  (bind _notifyname (Animation|Montage|PlayMontage (Variables|Character|GetMesh) "/Game/AITest/Enemies/AI/Animations/Melee/AM_Sheath_Sword.AM_Sheath_Sword")
    (:OnCompleted
      (Default|CallOnWeaponUnquipped))
    (:OnNotifyBegin
      (switch name _notifyname
        (:DropSword
          (Actor|DestroyActor (Variables|Default|GetWeaponActor))
          (Variables|Default|SetIsWieldingWeapon false))))))

(event EventAttack
  (bind _returnvalue (Transformation|GetActorLocation))
  (bind _notifyname (Animation|Montage|PlayMontage (Variables|Character|GetMesh) "/Game/AITest/Enemies/AI/Animations/Melee/AM_Attack.AM_Attack")
    (:then
      (Variables|/Game/AITest/DamageSystem/BPC_DamageSystem.BPC_DamageSystem_C|SetIsInterruptible (Variables|Default|GetBPC_DamageSystem) false))
    (:OnCompleted
      (Default|CallOnAttackEnd :!label _label)
      (Variables|/Game/AITest/DamageSystem/BPC_DamageSystem.BPC_DamageSystem_C|SetIsInterruptible (Variables|Default|GetBPC_DamageSystem) true))
    (:OnInterrupted
      (goto _label))
    (:OnNotifyBegin
      (switch name _notifyname
        (:Attack
          (bind (_outhit _returnvalue_2) (Collision|SphereTraceForObjects _returnvalue (+ _returnvalue (* (Transformation|GetActorForwardVector) 2e+02)) 2e+01 (Utilities|Array|MakeArray "ObjectTypeQuery3") false 0 "None"))
          (if _returnvalue_2
            (Class|BPIDamagable|TakeDamage(Message) (.HitActor (Collision|BreakHitResult _outhit)) (Utilities|Struct|MakeS_DamageInfo 3e+01 "NewEnumerator1"))))))))

(fn ConstructionScript
  (|CallParentFunction))